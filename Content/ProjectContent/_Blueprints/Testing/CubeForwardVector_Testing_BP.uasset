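; A test Blueprint that drives a cube continuously along its own forward vector while turning it.
; Each Tick adds TurningGear to the cube's world yaw, without delta-time scaling, then moves it forward by Speed times DeltaSeconds without sweep.
; The Turning event sets TurningGear from its Gear input, controlling the turn rate and direction.
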(event Custom|Turning
  (params (Gear :type Float%20%28single-precision%29))
  (Variables|Default|SetTurningGear Gear))

(event EventTick
  (params (DeltaSeconds :type Float%20%28single-precision%29))
  (bind _cube (Variables|Default|GetCube))
  (bind _cube_2 (Variables|Default|GetCube))
  (bind _returnvalue (Transformation|GetWorldRotation _cube))
  (Transformation|SetWorldRotation (Variables|Default|GetCube) (Math|Rotator|MakeRotator (.roll _returnvalue) (.pitch _returnvalue) (+ (.yaw _returnvalue) (Variables|Default|GetTurningGear))) false false)
  (Utilities|FlowControl|Sequence
    (:then_1
      (Transformation|SetWorldLocation (Variables|Default|GetCube) (+ (Transformation|GetWorldLocation _cube_2) (* (* (Math|Vector|GetForwardVector _cube_2) (Variables|Default|GetSpeed)) DeltaSeconds)) false false))))

(fn ConstructionScript)