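; Ship-mounted Harpoon missile launcher that automatically engages opposing-side pawns while its owner ship's missile system is active.
; Each tick it selects the nearest pawn within sensing range, beyond a minimum distance and in line of sight.
; A fire-rate check then triggers the first of two launch units not reloading.
; The server spawns a missile homing on the target and starts that unit's reload delay.
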(event Custom|FireUnit01
  (bind _arrow (Variables|Default|GetArrow))
  (bind _returnvalue (Transformation|GetWorldTransform _arrow))
  (if (Networking|IsServer)
    (Variables|Default|SetLastTimeOfFire (GameState|GetServerWorldTimeSeconds (Game|GetGameState)))
    (bind _returnvalue_2 (Game|SpawnActorfromClass "/Game/_ProjectContent/_Blueprints/Testing/Harpoon_Missile_BP.Harpoon_Missile_BP_C" (Math|Transform|MakeTransform (.location _returnvalue) (.rotation _returnvalue) "0.400000,0.400000,0.400000") "Undefined" 0 0))
    (Variables|/Game/_ProjectContent/_Blueprints/Testing/Harpoon_Missile_BP.Harpoon_Missile_BP_C|SetHomingTarget _returnvalue_2 (Actor|GetComponentbyClass (Variables|Default|GetTarget) "/Script/Engine.SceneComponent"))
    (CallFunction|Unit01Reload)))

(event Custom|EventUpdateOnServer
  (CallFunction|FindBestTarget)
  (Variables|Default|GetTarget
    (:then
      (CallFunction|UpdateFire))
    (:else)))

(event Custom|FireUnit02
  (bind _arrow1 (Variables|Default|GetArrow1))
  (bind _returnvalue (Transformation|GetWorldTransform _arrow1))
  (if (Networking|IsServer)
    (Variables|Default|SetLastTimeOfFire (GameState|GetServerWorldTimeSeconds (Game|GetGameState)))
    (bind _returnvalue_2 (Game|SpawnActorfromClass "/Game/_ProjectContent/_Blueprints/Testing/Harpoon_Missile_BP.Harpoon_Missile_BP_C" (Math|Transform|MakeTransform (.location _returnvalue) (.rotation _returnvalue) "0.400000,0.400000,0.400000") "Undefined" 0 0))
    (Variables|/Game/_ProjectContent/_Blueprints/Testing/Harpoon_Missile_BP.Harpoon_Missile_BP_C|SetHomingTarget _returnvalue_2 (Actor|GetComponentbyClass (Variables|Default|GetTarget) "/Script/Engine.SceneComponent"))
    (CallFunction|Unit02Reload)))

(event Custom|Unit02_Reload
  (Variables|Default|SetUnit2_Reload? true)
  (Utilities|FlowControl|Delay (Variables|Default|GetReloadTime))
  (Variables|Default|SetUnit2_Reload? false))

(event Custom|Unit01_Reload
  (Variables|Default|SetUnit1_Reload? true)
  (Utilities|FlowControl|Delay (Variables|Default|GetReloadTime))
  (Variables|Default|SetUnit1_Reload? false))

(event EventTick
  (params (DeltaSeconds :type Float%20%28single-precision%29))
  (bind _missilesystemstate (CallFunction|GetShipCommand (Variables|Default|GetShip_Owner)))
  (if _missilesystemstate
    (CallFunction|EventUpdateonServer)))

(fn ConstructionScript)

(fn FindBestTarget
  (bind _turret_base (Variables|Default|GetTurret_Base))
  (bind _returnvalue (Transformation|GetWorldLocation _turret_base))
  (LocalVariables|SetBestDistance%20%28Local%29 (+ (Variables|Default|GetSensingRange) 1.0))
  (bind _outactors (Collision|SphereOverlapActors (Transformation|GetActorLocation) (Variables|Default|GetSensingRange) (Utilities|Array|MakeArray "ObjectTypeQuery3") "/Script/Engine.Actor"))
  (for _array_element _outactors
    ;[1 1 1] Compare Ship Side
    (bind _shipside (CallFunction|GetShipSide _array_element))
    (if (Utilities|Enum|NotEqual(Enum) _shipside (Variables|Default|GetOwner_Side))
      (bind _output_get (LocalVariables|SetCurrentTarget%20%28Local%29 _array_element))
      (if (> (Transformation|GetDistanceTo _output_get self) (Variables|Default|GetCloseDistance))
        (bind _output_get_2 (LocalVariables|SetCurrentDistance%20%28Local%29 (Transformation|GetDistanceTo _output_get self)))
        (if (or (< _output_get_2 (LocalVariables|GetBestDistance%20%28Local%29)) (not (Utilities|IsValid (LocalVariables|GetBestTarget%20%28Local%29))))
          (bind _result (CallFunction|HasLineOfSight (Math|Vector|MakeVector (.x _returnvalue) (.y _returnvalue) 2.5e+02) (Transformation|GetActorLocation (LocalVariables|GetCurrentTarget%20%28Local%29)) (Utilities|Array|MakeArray self (LocalVariables|GetCurrentTarget%20%28Local%29))))
          (if _result
            (LocalVariables|SetBestTarget%20%28Local%29 (LocalVariables|GetCurrentTarget%20%28Local%29))
            (LocalVariables|SetBestDistance%20%28Local%29 (LocalVariables|GetCurrentDistance%20%28Local%29)))))))
  (Variables|Default|SetTarget (LocalVariables|GetBestTarget%20%28Local%29)))

(fn UpdateFire
  (if (> (- (Utilities|Time|GetGameTimeinSeconds) (Variables|Default|GetLastTimeOfFire)) (Variables|Default|GetRateOfFire))
    (if (not (Variables|Default|GetUnit1_Reload?))
      (CallFunction|FireUnit01)
      (elif (not (Variables|Default|GetUnit2_Reload?))
        (CallFunction|FireUnit02)))))

(fn OnRepShipSide)

(fn OnRepLastTimeOfFire)