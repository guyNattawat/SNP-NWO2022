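; Two-tube Harpoon missile launcher weapon that fires homing missiles at targets assigned per tube through SetTargetOnWeapon.
; While toggled on, Tick drives a one-second delayed update that lists opposing-side pawns in sensing range and reloads tubes whose missile is gone.
; Missiles spawn only on the server, with tube status and targets published in UnitWeaponStruct and launch Niagara effects triggered once per shot.
; The automatic best-target and rate-of-fire logic is present but disconnected.
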(event Custom|FireUnit01
  (params (Target_Unit1 :type Actor%20Object%20Reference))
  (Utilities|Struct|SetmembersinUnitWeaponStruct (Variables|Default|GetUnitWeapon_Struct) "Close" Target_Unit1)
  (if (Networking|IsServer)
    (bind _returnvalue (Game|SpawnActorfromClass "/Game/_ProjectContent/_Blueprints/Character/Weapon/Harpoon_Missile_BP.Harpoon_Missile_BP_C" (Math|Transform|MakeTransform (Transformation|GetSocketLocation (Variables|Default|GetTurret_Base) "FirePose") (.rotation (Transformation|GetWorldTransform (Variables|Default|GetArrow))) "0.100000,0.100000,0.100000") "Undefined" 0 0))
    (Variables|/Game/_ProjectContent/_Blueprints/Character/Weapon/Harpoon_Missile_BP.Harpoon_Missile_BP_C|SetHomingTarget _returnvalue (CallFunction|GetUnitSceneComponent[Unit] Target_Unit1))
    (Default|Spawned _returnvalue (Variables|Default|GetOwner_Side) self)
    (Utilities|Struct|SetmembersinUnitWeaponStruct (Variables|Default|GetUnitWeapon_Struct) "Homing")
    (Variables|Default|SetMissileUnit01_Ref _returnvalue)
    (Variables|Default|SetUnit1_Launched? true)))

(event Custom|EventUpdateOnServer
  (Utilities|FlowControl|Delay 1.0)
  (CallFunction|FindTargetinRange)
  (CallFunction|UpdateInfo)
  (CallFunction|MissileValidate))

(event Custom|FireUnit02
  (params (Target_Unit2 :type Actor%20Object%20Reference))
  (Utilities|Struct|SetmembersinUnitWeaponStruct (Variables|Default|GetUnitWeapon_Struct) "Close" Target_Unit2)
  (if (Networking|IsServer)
    (bind _returnvalue (Game|SpawnActorfromClass "/Game/_ProjectContent/_Blueprints/Character/Weapon/Harpoon_Missile_BP.Harpoon_Missile_BP_C" (Math|Transform|MakeTransform (Transformation|GetSocketLocation (Variables|Default|GetTurret_Base) "FirePose2") (.rotation (Transformation|GetWorldTransform (Variables|Default|GetArrow1))) "0.050000,0.050000,0.050000") "Undefined" 0 0))
    (Variables|/Game/_ProjectContent/_Blueprints/Character/Weapon/Harpoon_Missile_BP.Harpoon_Missile_BP_C|SetHomingTarget _returnvalue (CallFunction|GetUnitSceneComponent[Unit] Target_Unit2))
    (Default|Spawned _returnvalue (Variables|Default|GetOwner_Side) self)
    (Utilities|Struct|SetmembersinUnitWeaponStruct (Variables|Default|GetUnitWeapon_Struct) "Homing")
    (Variables|Default|SetMissileUnit02_Ref _returnvalue)
    (Variables|Default|SetUnit2_Launched? true)))

(event Custom|Unit02_Reload
  (Variables|Default|SetUnit2_Launched? false)
  (Utilities|Struct|SetmembersinUnitWeaponStruct (Variables|Default|GetUnitWeapon_Struct) "Reload")
  (Variables|Default|SetUnit2_Reload? true)
  (Utilities|FlowControl|Delay (Variables|Default|GetReloadTime))
  (Variables|Default|SetUnit2_Reload? false)
  (Utilities|Struct|SetmembersinUnitWeaponStruct (Variables|Default|GetUnitWeapon_Struct) "Ready"))

(event Custom|Unit01_Reload
  (Variables|Default|SetUnit1_Launched? false)
  (Utilities|Struct|SetmembersinUnitWeaponStruct (Variables|Default|GetUnitWeapon_Struct) "Reload")
  (Variables|Default|SetUnit1_Reload? true)
  (Utilities|FlowControl|Delay (Variables|Default|GetReloadTime))
  (Variables|Default|SetUnit1_Reload? false)
  (Utilities|Struct|SetmembersinUnitWeaponStruct (Variables|Default|GetUnitWeapon_Struct) "Ready"))

(event Custom|Update%20Info
  (Utilities|Struct|SetmembersinUnitWeaponStruct (Variables|Default|GetUnitWeapon_Struct) (Variables|Default|GetTargetInRange_Arr)))

(event Custom|SetTargetOnWeapon
  (params (TargetRef :type Actor%20Object%20Reference) (WeaponUnit :type Integer))
  (if (== WeaponUnit 1)
    (CallFunction|FireUnit01 TargetRef)
    (elif (== WeaponUnit 2)
      (CallFunction|FireUnit02 TargetRef))))

(event Custom|MissileValidate
  (Utilities|FlowControl|Sequence
    (:then_0
      (Utilities|IsValid (Variables|Default|GetMissileUnit01_Ref)
        (:Is%20Not%20Valid
          (if (Variables|Default|GetUnit1_Launched?)
            (CallFunction|Unit01Reload)))))
    (:then_1
      (Utilities|IsValid (Variables|Default|GetMissileUnit02_Ref)
        (:Is%20Not%20Valid
          (if (Variables|Default|GetUnit2_Launched?)
            (CallFunction|Unit02Reload)))))))

(event Custom|ToggleStatus
  (params (Status :type Boolean))
  (Utilities|Struct|SetmembersinUnitWeaponStruct (Variables|Default|GetUnitWeapon_Struct) Status))

(event Custom|UpdateVFX
  (Utilities|FlowControl|Sequence
    (:then_0
      (if (Variables|Default|GetUnit1_Launched?)
        (Utilities|FlowControl|DoOnce false :!label _label
          (:Completed
            (Components|Activation|SetActive (Variables|Default|GetNiagara) true true)))
        (else
          (goto _label Reset))))
    (:then_1
      (if (Variables|Default|GetUnit2_Launched?)
        (Utilities|FlowControl|DoOnce false :!label _label_2
          (:Completed
            (Components|Activation|SetActive (Variables|Default|GetNiagara1) true true)))
        (else
          (goto _label_2 Reset))))))

(event EventBeginPlay
  (Variables|Default|SetCurrentAmmo (Variables|Default|GetMaxAmmo))
  (Variables|Default|SetWeapon_Details_Struct (Utilities|Struct|MakeWeapon_Details_Struct self "Harpoon Block IC" (Variables|Default|GetWeaponStatus) (Variables|Default|GetCurrentAmmo) (Variables|Default|GetMaxAmmo) 0 2))
  (Utilities|Struct|SetmembersinUnitWeaponStruct (Variables|Default|GetUnitWeapon_Struct) "Ready" "Ready" true))

(event EventTick
  (params (DeltaSeconds :type Float%20%28single-precision%29))
  (if (Utilities|Struct|BreakUnitWeaponStruct (Variables|Default|GetUnitWeapon_Struct))
    (CallFunction|EventUpdateonServer)
    (CallFunction|UpdateVFX)))

(fn ConstructionScript)

(fn FindBestTarget
  (bind _turret_base (Variables|Default|GetTurret_Base))
  (bind _returnvalue (Transformation|GetWorldLocation _turret_base))
  (LocalVariables|SetBestDistance%20%28Local%29 (+ (Variables|Default|GetSensingRange) 1.0))
  (bind _outactors (Collision|SphereOverlapActors (Transformation|GetActorLocation) (Variables|Default|GetSensingRange) (Utilities|Array|MakeArray "ObjectTypeQuery3") "/Script/Engine.Actor"))
  (for _array_element _outactors
    ;[1 1 1] Compare Ship Side
    (bind _shipside (CallFunction|GetUnitSide[Unit] _array_element))
    (if (Utilities|Enum|NotEqual(Enum) _shipside (Variables|Default|GetOwner_Side))
      (bind _output_get (LocalVariables|SetCurrentTarget%20%28Local%29 _array_element))
      (if (> (Transformation|GetDistanceTo _output_get self) (Variables|Default|GetCloseDistance))
        (bind _output_get_2 (LocalVariables|SetCurrentDistance%20%28Local%29 (Transformation|GetDistanceTo _output_get self)))
        (if (or (< _output_get_2 (LocalVariables|GetBestDistance%20%28Local%29)) (not (Utilities|IsValid (LocalVariables|GetBestTarget%20%28Local%29))))
          (bind _result (CallFunction|HasLineOfSight (Math|Vector|MakeVector (.x _returnvalue) (.y _returnvalue) 2.5e+02) (Transformation|GetActorLocation (LocalVariables|GetCurrentTarget%20%28Local%29)) (Utilities|Array|MakeArray self (LocalVariables|GetCurrentTarget%20%28Local%29))))
          (if _result
            (LocalVariables|SetBestTarget%20%28Local%29 (LocalVariables|GetCurrentTarget%20%28Local%29))
            (LocalVariables|SetBestDistance%20%28Local%29 (LocalVariables|GetCurrentDistance%20%28Local%29)))))))
  (Variables|Default|SetTarget (LocalVariables|GetBestTarget%20%28Local%29)))

(fn UpdateFire
  (if (> (- (Utilities|Time|GetGameTimeinSeconds) (Variables|Default|GetLastTimeOfFire)) (Variables|Default|GetRateOfFire))
    (if (not (Variables|Default|GetUnit1_Reload?))
      (CallFunction|FireUnit01)
      (elif (not (Variables|Default|GetUnit2_Reload?))
        (CallFunction|FireUnit02)))))

(fn OnRepShipSide)

(fn OnRepLastTimeOfFire)

(fn FindTargetinRange
  (Utilities|Array|Clear (Variables|Default|GetTargetInRange_Arr))
  (bind _outactors (Collision|SphereOverlapActors (Transformation|GetActorLocation) (Variables|Default|GetSensingRange) (Utilities|Array|MakeArray "ObjectTypeQuery3") "/Script/Engine.Actor"))
  (for _array_element _outactors
    (bind (_shipside _characterref) (CallFunction|GetUnitSide[Unit] _array_element))
    (if (Utilities|Enum|NotEqual(Enum) _shipside (Variables|Default|GetOwner_Side))
      (Utilities|Array|AddUnique (Variables|Default|GetTargetInRange_Arr) _characterref))))