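; World map capture actor that frames the area between two corner actors, UpperLeft and LowerRight, with its scene capture component.
; When both references are valid, the Construction Script moves the actor to their XY midpoint and keeps its own height.
; It sets the capture's OrthoWidth to the larger of the X and Y spans, so a square frame covers both corners.
; The event graph holds no runtime logic.
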(event EventBeginPlay)

(fn ConstructionScript
  (bind _upperleft (Variables|Default|GetUpperLeft))
  (bind _lowerright (Variables|Default|GetLowerRight))
  (bind _lowerright_2 (Variables|Default|GetLowerRight))
  (bind _upperleft_2 (Variables|Default|GetUpperLeft))
  (bind _returnvalue (Transformation|GetActorLocation _lowerright_2))
  (bind _returnvalue_2 (Transformation|GetActorLocation _upperleft))
  (bind _returnvalue_3 (Transformation|GetActorLocation _lowerright))
  (bind _returnvalue_4 (Transformation|GetActorLocation _upperleft_2))
  (bind _returnvalue_5 (- _returnvalue_3 _returnvalue_2))
  (bind _returnvalue_6 (/ _returnvalue_5 2.0))
  (bind _returnvalue_7 (+ _returnvalue_2 _returnvalue_6))
  (bind (_x _y) (Math|Vector|BreakVector _returnvalue_7))
  (Utilities|IsValid _upperleft
    (:Is%20Valid
      (Utilities|IsValid _lowerright
        (:Is%20Valid
          (Transformation|SetActorLocation (Math|Vector|MakeVector _x _y (.z (Transformation|GetActorLocation))) false true)
          (Variables|/Script/Engine.SceneCaptureComponent2D|SetOrthoWidth (Variables|Default|GetSceneCapture) (Math|Float|Max(Float) (Math|Float|Absolute(Float) (- (.x _returnvalue) (.x _returnvalue_4))) (Math|Float|Absolute(Float) (- (.y _returnvalue) (.y _returnvalue_4))))))))))