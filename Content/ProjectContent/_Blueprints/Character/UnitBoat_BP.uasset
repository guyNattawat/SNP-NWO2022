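; RTS boat unit with a child turret, clickable selection decal and a team side stored in OwnerSide and the actor tag.
; On BeginPlay it caches its AI controller and makes the turret ignore it and share its side.
; Client clicks toggle its membership in the RTSController selection.
; MoveToLocation uses a timeline to push the boat along its mesh axis while turning toward the blackboard TargetLocation, then hands off to UnitAIController.
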(event OnComponentBeginOverlap(CapsuleComponent)
  (params (OverlappedComponent :type Primitive%20Component%20Object%20Reference) (OtherActor :type Actor%20Object%20Reference) (OtherComp :type Primitive%20Component%20Object%20Reference) (OtherBodyIndex :type Integer) (bFromSweep :type Boolean) (SweepResult :type Hit%20Result%20Structure%20%28by%20ref%29)))

(event Custom|IsSelected
  (params (IsSelected :type Boolean))
  ;[1 1 1] If AI Selected it will Visibility
  (Rendering|SetVisibility (Variables|Default|GetDecal) IsSelected false))

(event Custom|SET%20OwnerSide
  (params (OwnerSide :type String))
  ;[1 1 1] Set Owner Side
  (bind _output_get (Variables|Default|SetOwnerSide OwnerSide))
  (Variables|Default|SetTags (Utilities|Array|MakeArray (Utilities|String|StringToName _output_get)))
  (CallFunction|SETOwnerSideonClient _output_get))

(event Custom|CreateLine
  ;[1 1 1] Create Line for Measure Forward Actor BT Boat and Rotate Measure
  (if (Utilities|IsValid (Variables|Default|GetRotateMeasure))
    (Actor|DestroyActor (Variables|Default|GetRotateMeasure)))
  (bind _returnvalue (Game|SpawnActorfromClass "/Game/ProjectContent/_Blueprints/Character/RotateMeasure_BP.RotateMeasure_BP_C" (Math|Transform|MakeTransform (Variables|Default|GetDestinationLocation) "0, 0, 0" "1,1,1") "Undefined" 0 0))
  (Variables|Default|SetRotateMeasure _returnvalue)
  (Transformation|SetWorldRotation (Variables|/Script/Engine.Actor|GetRootComponent _returnvalue) (Math|Rotator|MakeRotator (.roll (Math|Rotator|FindLookatRotation (Transformation|GetWorldLocation (Variables|/Script/Engine.Actor|GetRootComponent _returnvalue)) (Transformation|GetActorLocation))) (.pitch (Math|Rotator|FindLookatRotation (Transformation|GetWorldLocation (Variables|/Script/Engine.Actor|GetRootComponent _returnvalue)) (Transformation|GetActorLocation))) (.yaw (Math|Rotator|FindLookatRotation (Transformation|GetWorldLocation (Variables|/Script/Engine.Actor|GetRootComponent _returnvalue)) (Transformation|GetActorLocation)))) false false))

(event Custom|SET%20OwnerSide%20On%20Client
  (params (OwnerSide :type String))
  (bind _output_get (Variables|Default|SetOwnerSide OwnerSide))
  (Variables|Default|SetTags (Utilities|Array|MakeArray (Utilities|String|StringToName _output_get))))

(event Custom|AIMoveToLocation
  (bind _self self)
  ;[1 1 1] AI MoveTo on Server Side
  (AI|AIMoveTo _self (AI|Components|Blackboard|GetValueasVector (AI|GetBlackboard _self) (Utilities|Name|MakeLiteralName "TargetLocation")) 0 5.0 false))

(event Custom|GET%20OwnerSide
  (Development|PrintString (Variables|Default|GetOwnerSide)))

(event Custom|MoveToLocation
  (bind _capsulecomponent (Variables|Collision|GetCapsuleComponent))
  (bind _returnvalue (Transformation|GetWorldRotation _capsulecomponent))
  ;[1 1 1] AI Rotate and Move Forward Following Forward Vector
  (Utilities|FlowControl|Sequence
    (:then_0
      (Components|Timeline|SetPlayRate (Variables|Default|GetRotateToLocation) 1.0)
      (bind _newtrack_0 (Timeline|RotateToLocation PlayFromStart)
        (:Update
          (Transformation|SetWorldLocation (Variables|Collision|GetCapsuleComponent) (+ (Transformation|GetWorldLocation (Variables|Collision|GetCapsuleComponent)) (* (* (* (Math|Vector|GetForwardVector (Variables|Character|GetMesh)) "-1.000000,-1.000000, 0") 1e+02) (Utilities|Time|GetWorldDeltaSeconds))) false false)
          (Transformation|SetWorldRotation (Variables|Collision|GetCapsuleComponent) (Math|Rotator|Lerp(Rotator) (Math|Rotator|MakeRotator (.roll _returnvalue) (.pitch _returnvalue) (.yaw _returnvalue)) (Math|Rotator|MakeRotator (.roll _returnvalue) (.pitch _returnvalue) (.yaw (Math|Rotator|FindLookatRotation (Transformation|GetWorldLocation _capsulecomponent) (AI|Components|Blackboard|GetValueasVector (AI|GetBlackboard self) (Utilities|Name|MakeLiteralName "TargetLocation"))))) (/ _newtrack_0 3e+01) true) false false))
        (:Finished
          (Variables|Default|SetCheckFirst? false)
          (bind _asunit_aicontroller (Utilities|Casting|CastToUnitAIController (AI|GetAIController self)))
          (Default|AIMovetoonServer _asunit_aicontroller))))
    (:then_1
      (if (not (Variables|Default|GetCheckFirst?))
        (Class|NavMovementComponent|StopActiveMovement (Variables|Character|GetCharacterMovement))))))

(event EventBeginPlay
  (Utilities|FlowControl|Sequence
    (:then_0
      (Networking|ForceNetUpdate)
      (Variables|Default|SetAIController_Ref (AI|GetAIController self)))
    (:then_1
      (bind _asturret_bp_test (Utilities|Casting|CastToTurret_BP_test (Variables|/Script/Engine.ChildActorComponent|GetChildActor (Variables|Default|GetTurret_BP_test))))
      (Utilities|Array|AddUnique (Variables|/Game/ProjectContent/_Blueprints/Testing/Turret_BP_test.Turret_BP_test_C|GetActors%20to%20Ignore%20Arr _asturret_bp_test) self)
      (Variables|/Game/ProjectContent/_Blueprints/Testing/Turret_BP_test.Turret_BP_test_C|SetOwnerSide _asturret_bp_test (Variables|Default|GetOwnerSide)))))

(event MouseInput|EventActorOnClicked
  (params (ButtonPressed :type Key%20Structure :default "None"))
  ;[1 1 1] When Actor OnClicked It will Visible / Hidden Decal and Add / Remove Unit from Selection Array
  (if (== ButtonPressed "LeftMouseButton")
    (Networking|SwitchHasAuthority
      (:Remote
        (bind _asrtscontroller (Utilities|Casting|CastToRTSController (Game|GetPlayerController 0)))
        (if (Rendering|IsVisible (Variables|Default|GetDecal))
          (Default|RemovUnitfromSelection _asrtscontroller self)
          (else
            (Default|AddUnittoSelection _asrtscontroller self)))))))

(event EventTick
  (params (DeltaSeconds :type Float%20%28single-precision%29))
  (bind _asturret_bp_test (Utilities|Casting|CastToTurret_BP_test (Variables|/Script/Engine.ChildActorComponent|GetChildActor (Variables|Default|GetTurret_BP_test)))))

(fn ConstructionScript)

(fn SetActorMaterial)

(fn OnRepOwnerSide
  (CallFunction|SetActorMaterial))

(fn PrintClientSide
  (return (Variables|Default|GetOwnerSide)))