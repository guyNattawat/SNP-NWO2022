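; OTO Melara 40L70mm twin-barrel ship turret that engages an externally assigned target and reports status through a weapon struct.
; While toggled on, Tick lists other-side units in range, turns the yaw-clamped turret and pitches the barrel using a low-arc ballistic solution.
; When cooled down and aligned, it alternates muzzles, spawning shells on the server with velocity-dependent spread, and reloads after a delay when empty.
; FindBestTarget is never called.
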(event Custom|EventUpdateOnServer
  (params (DeltaSec :type Float%20%28single-precision%29))
  (CallFunction|FindTargetinRange)
  (CallFunction|UpdateInfo)
  (Variables|Private|GetTarget
    (:then
      (Private|UpdateFire))
    (:else)))

(event Custom|Reload
  ;[1 1 1] Reload
  (Utilities|Struct|SetmembersinUnitWeaponStruct (Variables|Default|GetUnitWeapon_Struct) "Reload")
  (Variables|Default|SetReload? true)
  (Utilities|Struct|SetmembersinUnitWeaponStruct (Variables|Default|GetUnitWeapon_Struct) "Reload")
  (Utilities|FlowControl|Delay (Variables|Ability|GetReloadSpeed))
  (Variables|Ability|SetCurrentAmmo (Variables|Ability|GetMaxAmmo))
  (Variables|Default|SetReload? false)
  (Utilities|Struct|SetmembersinUnitWeaponStruct (Variables|Default|GetUnitWeapon_Struct) "Ready"))

(event Custom|ToggleStatus
  (params (Status :type Boolean))
  (Utilities|Struct|SetmembersinUnitWeaponStruct (Variables|Default|GetUnitWeapon_Struct) Status))

(event Custom|FireOnServer
  (params (FirePose :type Arrow%20Component%20Object%20Reference) (FirePoseLocation :type Vector))
  ;[1 1 1] Fire On Server
  (Utilities|Struct|SetmembersinUnitWeaponStruct (Variables|Default|GetUnitWeapon_Struct) "Attacking" (Variables|Private|GetTarget))
  (if (> (Variables|Ability|GetCurrentAmmo) 0)
    (Variables|Ability|SetCurrentAmmo (- (Variables|Ability|GetCurrentAmmo) 1))
    (if (Networking|IsServer)
      (Variables|Private|SetTimeOfLastFire (GameState|GetServerWorldTimeSeconds (Game|GetGameState)))
      (Utilities|FlowControl|Sequence
        (:then_0
          (if (> (.x (Transformation|GetVelocity (Variables|Default|GetShip_Owner))) 0.0)
            (Variables|Ability|SetAccuracy 0.3)
            (else
              (Variables|Ability|SetAccuracy 0.5)))
          (Game|SpawnActorfromClass "/Game/_ProjectContent/_Blueprints/Character/Weapon/44mmShell.44mmShell_C" (Math|Transform|MakeTransform FirePoseLocation (Math|Conversions|RotationFromXVector (Math|Random|RandomUnitVectorinConeinDegrees (Math|Vector|GetForwardVector FirePose) (Variables|Ability|GetAccuracy))) "0.050000,0.050000,0.050000") "Undefined" 0 0))
        (:then_1
          (CallFunction|FireVFX))))
    (elif (not (Variables|Default|GetReload?))
      (CallFunction|Reload))))

(event Custom|Update%20Info
  ;[1 1 1] Update Weapon Info
  (Utilities|Struct|SetmembersinUnitWeaponStruct (Variables|Default|GetUnitWeapon_Struct) (Variables|Default|GetTargetInRange_Arr)))

(event Custom|SetTargetOnWeapon
  (params (TargetRef :type Character%20Object%20Reference))
  ;[1 1 1] Set Target On Weapon
  (Variables|Private|SetTarget TargetRef))

(event Custom|Turret%20Fire%20Control
  (bind _turret_barrel (Variables|Default|Getturret_Barrel))
  (Utilities|FlowControl|FlipFlop
    (:A
      (CallFunction|FireonServer (Variables|Default|GetFirePos1) (Transformation|GetSocketLocation _turret_barrel "FirePose")))
    (:B
      (CallFunction|FireonServer (Variables|Default|GetFirePos2) (Transformation|GetSocketLocation _turret_barrel "FirePose2")))))

(event Custom|FireVFX
  (bind _firepos1 (Variables|Default|GetFirePos1))
  (bind _returnvalue (Transformation|GetSocketLocation _firepos1 "None"))
  (Niagara|SpawnSystematLocation "/Game/_ProjectContent/_Blueprints/VFX/N_TurretFire.N_TurretFire" _returnvalue "0, 0, 0" "0.300000,0.300000,0.300000")
  (Effects|SpawnEmitteratLocation "/Game/StarterContent/Particles/P_Explosion.P_Explosion" _returnvalue "0, 0, 0" "0.060000,0.060000,0.060000"))

(event EventBeginPlay
  (Variables|Ability|SetCurrentAmmo (Variables|Ability|GetMaxAmmo))
  (Variables|Default|SetWeapon_Details_Struct (Utilities|Struct|MakeWeapon_Details_Struct self "OTO Melara 40L70mm" (Variables|Default|GetStatus) (Variables|Ability|GetCurrentAmmo) (Variables|Ability|GetMaxAmmo) 0 1))
  (Utilities|Struct|SetmembersinUnitWeaponStruct (Variables|Default|GetUnitWeapon_Struct) "Ready" true))

(event EventTick
  (params (DeltaSeconds :type Float%20%28single-precision%29))
  (Utilities|FlowControl|Sequence
    (:then_0
      (if (Utilities|Struct|BreakUnitWeaponStruct (Variables|Default|GetUnitWeapon_Struct))
        (CallFunction|EventUpdateonServer DeltaSeconds)
        (Variables|Private|GetTarget
          (:then
            (Private|UpdateTurretRotation DeltaSeconds))
          (:else))))))

(fn ConstructionScript)

(fn FindBestTarget
  (bind _turret_top (Variables|Default|Getturret_Top))
  (bind _returnvalue (Transformation|GetWorldLocation _turret_top))
  (Utilities|FlowControl|Sequence
    (:then_0
      (LocalVariables|SetBestDistance%20%28Local%29 (+ (Variables|Contants|GetSensingRange) 1.0))
      (bind _outactors (Collision|SphereOverlapActors (Transformation|GetActorLocation) (Variables|Contants|GetSensingRange) (Utilities|Array|MakeArray "ObjectTypeQuery3") "/Script/Engine.Actor" (Variables|Default|GetActors%20to%20Ignore%20Arr)))
      ;[1 1 1] Compare Client Side
      (for _array_element _outactors
        (bind _shipside (CallFunction|GetUnitSide[Unit] _array_element))
        (if (Utilities|Enum|NotEqual(Enum) _shipside (Variables|Default|GetOwnerSide))
          (bind _output_get (LocalVariables|SetCurrentTarget%20%28Local%29 _array_element))
          (bind _output_get_2 (LocalVariables|SetCurrentDistance%20%28Local%29 (Transformation|GetDistanceTo _output_get self)))
          (if (or (< _output_get_2 (LocalVariables|GetBestDistance%20%28Local%29)) (not (Utilities|IsValid (LocalVariables|GetBestTarget%20%28Local%29)))) ; Is This closest target so far?
            (bind _result (CallFunction|HasLineOfSight (Math|Vector|MakeVector (.x _returnvalue) (.y _returnvalue) 3e+01) (Math|Vector|MakeVector (.x (Transformation|GetActorLocation (LocalVariables|GetCurrentTarget%20%28Local%29))) (.y (Transformation|GetActorLocation (LocalVariables|GetCurrentTarget%20%28Local%29))) 7e+01) (Variables|Default|GetActors%20to%20Ignore%20Arr)))
            (if _result
              (LocalVariables|SetBestTarget%20%28Local%29 (LocalVariables|GetCurrentTarget%20%28Local%29))
              (LocalVariables|SetBestDistance%20%28Local%29 (LocalVariables|GetCurrentDistance%20%28Local%29))))))
      (Variables|Private|SetTarget 0))))

(fn UpdateTurretRotation
  (params (DeltaSeconds :type Float%20%28single-precision%29))
  (bind _turret_base (Variables|Default|Getturret_Base))
  (bind _rotation_speed (Variables|Ability|GetRotation%20Speed))
  (bind _turret_barrel (Variables|Default|Getturret_Barrel))
  (bind _turret_barrel_2 (Variables|Default|Getturret_Barrel))
  (bind _target (Variables|Private|GetTarget))
  (bind _deltaseconds (LocalVariables|GetDeltaseconds))
  (bind _returnvalue (Transformation|GetSocketLocation _turret_barrel "FireSocket"))
  (bind _returnvalue_2 (Transformation|GetWorldTransform _turret_base))
  (bind _returnvalue_3 (Transformation|GetWorldRotation _turret_barrel_2))
  (bind _returnvalue_4 (Transformation|GetSocketRotation _turret_barrel "None"))
  (bind _mesh (Variables|/Script/Engine.Character|GetMesh _target))
  (bind _returnvalue_5 (Transformation|GetWorldLocation _mesh))
  (bind _returnvalue_6 (Math|Rotator|FindLookatRotation _returnvalue _returnvalue_5))
  (bind _returnvalue_7 (Class|KismetMathLibrary|RInterptoConstant _returnvalue_4 _returnvalue_6 _deltaseconds _rotation_speed))
  (bind _returnvalue_8 (Math|Transform|InverseTransformRotation _returnvalue_2 _returnvalue_7))
  (Transformation|SetRelativeRotation (Variables|Default|Getturret_Top) (Math|Rotator|MakeRotator (.roll _returnvalue_8) 0.0 (Math|Float|ClampAngle (.yaw _returnvalue_8) -9e+01 9e+01)) false false)
  (bind _angleresult (CallFunction|FindAngle))
  (Transformation|SetWorldRotation _turret_barrel_2 (Math|Rotator|MakeRotator (.roll _returnvalue_3) _angleresult (.yaw _returnvalue_3)) false false))

(fn OnRepOwnerSide)

(fn TurretColorSet)

(fn UpdateFire
  (if (> (- (Utilities|Time|GetGameTimeinSeconds) (Variables|Private|GetTimeOfLastFire)) (Variables|Private|GetRateOfFire)) ; Have Rate of Fire Cooled Down?
    (if (> (Math|Vector|DotProduct (Math|Vector|GetUnitDirection(Vector) (Transformation|GetWorldLocation (Variables|Default|Getturret_Top)) (Transformation|GetActorLocation (Variables|Private|GetTarget))) (Math|Vector|GetForwardVector (Variables|Default|Getturret_Top))) 0.99) ; Is the turret facing to target?
      (CallFunction|TurretFireControl))))

(fn FindAngle
  (bind _target (Variables|Private|GetTarget))
  (bind _velocity (Variables|Ability|GetVelocity))
  (bind _gravity (Variables|Ability|GetGravity))
  (bind _turret_barrel (Variables|Default|Getturret_Barrel))
  (bind _returnvalue (Transformation|GetSocketLocation _turret_barrel "FireSocket"))
  (bind _returnvalue_2 (Math|Float|Square _velocity))
  (bind _mesh (Variables|/Script/Engine.Character|GetMesh _target))
  (bind _returnvalue_3 (Math|Float|Square _returnvalue_2))
  (bind _returnvalue_4 (Transformation|GetWorldLocation _mesh))
  (bind _returnvalue_5 (- (.x _returnvalue_4) (.x _returnvalue)))
  (bind _returnvalue_6 (- (.y _returnvalue_4) (.y _returnvalue)))
  (bind _returnvalue_7 (+ (.z _returnvalue_4) 1e+01))
  (bind _returnvalue_8 (- _returnvalue_7 (.z _returnvalue)))
  (bind _returnvalue_9 (Math|Vector2D|Vector2DLength (Math|Vector2D|MakeVector2D _returnvalue_5 _returnvalue_6)))
  (bind _returnvalue_10 (Math|Float|Square _returnvalue_9))
  (bind _returnvalue_11 (* _returnvalue_8 _returnvalue_2))
  (bind _returnvalue_12 (* _returnvalue_9 _gravity))
  (bind _returnvalue_13 (* _returnvalue_10 _gravity))
  (bind _returnvalue_14 (* _returnvalue_11 2.0))
  (bind _returnvalue_15 (+ _returnvalue_13 _returnvalue_14))
  (bind _returnvalue_16 (* _returnvalue_15 _gravity))
  (bind _returnvalue_17 (- _returnvalue_3 _returnvalue_16))
  (bind _returnvalue_18 (Math|Float|Sqrt _returnvalue_17))
  (return (Math|Float|Min(Float) (Class|KismetMathLibrary|DegAtan (/ (+ _returnvalue_18 _returnvalue_2) _returnvalue_12)) (Class|KismetMathLibrary|DegAtan (/ (- _returnvalue_2 _returnvalue_18) _returnvalue_12)))))

(fn OnRepTimeOfLastFire)

(fn GetShipCommand
  (params (Ship%20Ref :type Character%20Object%20Reference)))

(fn FindTargetinRange
  (Utilities|Array|Clear (Variables|Default|GetTargetInRange_Arr))
  (bind _outactors (Collision|SphereOverlapActors (Transformation|GetActorLocation) (Variables|Contants|GetSensingRange) (Utilities|Array|MakeArray "ObjectTypeQuery3") "/Script/Engine.Actor"))
  (for _array_element _outactors
    (bind (_shipside _characterref) (CallFunction|GetUnitSide[Unit] _array_element))
    (if (Utilities|Enum|NotEqual(Enum) _shipside (Variables|Default|GetOwnerSide))
      (Utilities|Array|AddUnique (Variables|Default|GetTargetInRange_Arr) _characterref))))