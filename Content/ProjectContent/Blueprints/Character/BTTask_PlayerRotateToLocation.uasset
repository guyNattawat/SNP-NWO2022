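; Behavior tree task that steers a UnitBoat_BP pawn toward the blackboard's TargetLocation.
; Each execution nudges the capsule horizontally along the mesh's negated forward vector, scaled by delta time, without sweeping.
; It then snaps the capsule's yaw to the look-at angle plus a small offset, keeping pitch and roll, and finishes immediately with success.
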(event EventReceiveExecuteAI
  (params (OwnerController :type AI%20Controller%20Object%20Reference) (ControlledPawn :type Pawn%20Object%20Reference))
  (bind _asunit_boat_bp (Utilities|Casting|CastToUnitBoat_BP ControlledPawn))
  (Transformation|SetWorldLocation (Variables|/Script/Engine.Character|GetCapsuleComponent _asunit_boat_bp) (+ (Transformation|GetWorldLocation (Variables|/Script/Engine.Character|GetCapsuleComponent _asunit_boat_bp)) (* (* (* (Math|Vector|GetForwardVector (Variables|/Script/Engine.Character|GetMesh _asunit_boat_bp)) "-1.000000,-1.000000, 0") 1e+02) (Utilities|Time|GetWorldDeltaSeconds))) false false)
  (Transformation|SetWorldRotation (Variables|/Script/Engine.Character|GetCapsuleComponent _asunit_boat_bp) (Math|Rotator|MakeRotator (.roll (Transformation|GetWorldRotation (Variables|/Script/Engine.Character|GetCapsuleComponent _asunit_boat_bp))) (.pitch (Transformation|GetWorldRotation (Variables|/Script/Engine.Character|GetCapsuleComponent _asunit_boat_bp))) (+ (.yaw (Math|Rotator|FindLookatRotation (Transformation|GetWorldLocation (Variables|/Script/Engine.Character|GetCapsuleComponent _asunit_boat_bp)) (AI|Components|Blackboard|GetValueasVector (AI|GetBlackboard OwnerController) (Utilities|Name|MakeLiteralName "TargetLocation")))) 0.1)) false false)
  (AI|BehaviorTree|FinishExecute true))