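; Enemy AI boat Blueprint that moves and steers itself by setting its mesh transform every Tick.
; It moves horizontally along the mesh's reversed forward vector, scaled by Speed and delta time, without sweep.
; A Turning event, noted as coming from a controller widget, sets TurningGear, which is added to yaw each frame without delta-time scaling.
; An unconnected debug chain of timelines prints points on a unit circle.
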(event Custom|Turning
  (params (Gear :type Float%20%28single-precision%29))
  ;[1 1 1] Set Turning Gear [From : Controller Widget]
  (Variables|Default|SetTurningGear Gear))

(event EventBeginPlay
  ;[1 1 1] Set Location
  (Variables|Default|SetLocation (Transformation|GetWorldLocation (Variables|Character|GetMesh))))

(event EventTick
  (params (DeltaSeconds :type Float%20%28single-precision%29))
  (bind _mesh (Variables|Character|GetMesh))
  (bind _returnvalue (Transformation|GetWorldRotation _mesh))
  ;[1 1 1] Set Boat WorldLocation and WorldRotation
  (Utilities|FlowControl|Sequence
    (:then_0
      (bind _output_get (Variables|Default|SetLocation (+ (Transformation|GetWorldLocation (Variables|Character|GetMesh)) (* (* (* (Math|Vector|GetForwardVector (Variables|Character|GetMesh)) "-1.000000,-1.000000,0.000000") (Variables|Default|GetSpeed)) DeltaSeconds))))
      (Transformation|SetWorldLocation (Variables|Character|GetMesh) _output_get false false))
    (:then_1
      (Transformation|SetWorldRotation (Variables|Character|GetMesh) (Math|Rotator|MakeRotator (.roll _returnvalue) (.pitch _returnvalue) (+ (.yaw _returnvalue) (Variables|Default|GetTurningGear))) false false))))

(fn ConstructionScript)