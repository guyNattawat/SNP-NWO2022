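; Enemy AI boat that moves its Navigator component in a straight line, with no steering or decision logic in its graph.
; BeginPlay caches the Navigator's location, then Tick advances it by a stored forward vector, speed and delta time and teleport-free sets it without sweep.
; Three chained timelines compute semicircle arc points from the unit-circle equation, but only print them, leaving movement unaffected.
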(event EventBeginPlay
  ;[1 1 1] Set Location
  (Variables|Default|SetLocation (Transformation|GetWorldLocation (Variables|Default|GetNavigator)))
  (Components|Timeline|SetPlayRate (Variables|Default|GetFloatTime) 1.0)
  (bind _newtrack_0 (Timeline|FloatTime PlayFromStart)
    (:Update
      (Development|PrintString (Utilities|String|ToString(Vector) (Math|Vector|MakeVector _newtrack_0 (Math|Float|Sqrt (- 1.0 (* _newtrack_0 _newtrack_0))) 0.0))))
    (:Finished
      (Components|Timeline|SetPlayRate (Variables|Default|GetFloatTimeP2) 1.0)
      (bind _newtrack_0_2 (Timeline|FloatTimeP2 PlayFromStart)
        (:Update
          (Development|PrintString (Utilities|String|ToString(Vector) (Math|Vector|MakeVector _newtrack_0_2 (* (Math|Float|Sqrt (- 1.0 (* _newtrack_0_2 _newtrack_0_2))) -1.0) 0.0))))
        (:Finished
          (bind _newtrack_0_3 (Timeline|FloatTimeP3 PlayFromStart)
            (:Update
              (Development|PrintString (Utilities|String|ToString(Vector) (Math|Vector|MakeVector _newtrack_0_3 (Math|Float|Sqrt (- 1.0 (* _newtrack_0_3 _newtrack_0_3))) 0.0))))))))))

(event EventTick
  (params (DeltaSeconds :type Float%20%28single-precision%29))
  ;[1 1 1] Set BoatWorld Location
  (Utilities|FlowControl|Sequence
    (:then_0
      (bind _output_get (Variables|Default|SetLocation (+ (Variables|Default|GetLocation) (* (* (Variables|Default|GetActorForwardVector) (Variables|Default|GetSpeed)) DeltaSeconds))))
      (Transformation|SetWorldLocation (Variables|Default|GetNavigator) _output_get false false))))

(fn ConstructionScript)