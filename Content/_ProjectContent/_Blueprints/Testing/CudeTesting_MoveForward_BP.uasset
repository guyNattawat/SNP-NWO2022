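; Test actor that moves itself forward at a set speed and tracks overlap with AI enemy boats.
; Each tick it advances a stored location along ActorForwardVector without sweeping, then resets relative rotation, feeding that vector's X and Y into roll and pitch with zero yaw.
; Sphere begin and end overlaps with EnemyAIBoat_BP toggle an OverlappingAI flag, which this graph never reads.
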(event OnComponentBeginOverlap(Sphere)
  (params (OverlappedComponent :type Primitive%20Component%20Object%20Reference) (OtherActor :type Actor%20Object%20Reference) (OtherComp :type Primitive%20Component%20Object%20Reference) (OtherBodyIndex :type Integer) (bFromSweep :type Boolean) (SweepResult :type Hit%20Result%20Structure%20%28by%20ref%29))
  (Utilities|Casting|CastToEnemyAIBoat_BP OtherActor)
  (Variables|Default|SetOverlappingAI? true))

(event OnComponentEndOverlap(Sphere)
  (params (OverlappedComponent :type Primitive%20Component%20Object%20Reference) (OtherActor :type Actor%20Object%20Reference) (OtherComp :type Primitive%20Component%20Object%20Reference) (OtherBodyIndex :type Integer))
  (Utilities|Casting|CastToEnemyAIBoat_BP OtherActor)
  (Variables|Default|SetOverlappingAI? false))

(event EventTick
  (params (DeltaSeconds :type Float%20%28single-precision%29))
  (bind _actorforwardvector (Variables|Default|GetActorForwardVector))
  (bind (_x _y) (Math|Vector|BreakVector _actorforwardvector))
  (bind _output_get (Variables|Default|SetLocation (+ (Variables|Default|GetLocation) (* (* (Variables|Default|GetActorForwardVector) (Variables|Default|GetSpeed)) DeltaSeconds))))
  (Transformation|SetActorLocation _output_get false false)
  (Transformation|SetActorRelativeRotation (Math|Rotator|MakeRotator _x _y 0.0)))

(event EventBeginPlay
  (Variables|Default|SetLocation (Transformation|GetActorLocation)))

(fn ConstructionScript)