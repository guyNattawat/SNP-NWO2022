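; AI controller for boat units that starts their behavior tree and relays movement and state calls to the boat.
; On spawn it runs UnitBehavior_BT and passes the owner side to the UnitBoat_BP found through its Instigator.
; Two move events call the boat's regular and AI move functions only with authority.
; A checker event sets a test flag on that boat without an authority check, ignoring its BoatRef input.
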(event Custom|MoveToOnServer
  ;[1 1 1] MoveTo function
  (Networking|SwitchHasAuthority
    (:Authority
      (bind _asunit_boat_bp (Utilities|Casting|CastToUnitBoat_BP (Game|GetInstigator)))
      (Default|MovetoLocation _asunit_boat_bp))))

(event Custom|AIMoveToOnServer
  ;[1 1 1] MoveTo function
  (Networking|SwitchHasAuthority
    (:Authority
      (bind _asunit_boat_bp (Utilities|Casting|CastToUnitBoat_BP (Game|GetInstigator)))
      (Default|AIMovetoLocation _asunit_boat_bp))))

(event Custom|Spawned
  (params (OwnerSide :type String))
  ;[1 1 1] Event after Boat Spawn
  (AI|RunBehaviorTree "/Game/ProjectContent/Blueprints/Character/UnitBehavior_BT.UnitBehavior_BT")
  (bind _asunit_boat_bp (Utilities|Casting|CastToUnitBoat_BP (Game|GetInstigator)))
  (Default|SETOwnerSide _asunit_boat_bp OwnerSide))

(event Custom|SET%20CheckerVal%20OnServer
  (params (bool :type Boolean) (Boat%20Ref :type Unit%20Boat%20BP%20Object%20Reference))
  ;[1 1 1] SET CheckerVal OnServer
  (bind _asunit_boat_bp (Utilities|Casting|CastToUnitBoat_BP (Game|GetInstigator)))
  (Variables|/Game/ProjectContent/Blueprints/Character/UnitBoat_BP.UnitBoat_BP_C|SetCheckerTestVal01 _asunit_boat_bp bool))

(fn ConstructionScript)