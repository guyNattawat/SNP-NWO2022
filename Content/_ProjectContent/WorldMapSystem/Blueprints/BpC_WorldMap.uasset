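; World map component that shows ships, missiles and compounds as flag widgets on a zoomable RTS map.
; It converts between world and map coordinates using two corner bounds, repositioning flags and resizing ship flags on Tick.
; Add events create widgets through the map widget and hand references back to their actors, while visibility updates hide other-side units out of range.
; Map clicks are traced down to world locations where the controller spawns units.
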(event Custom|Initialize%20Map
  (params (WorldMap_WG :type World%20Map%20System%20Main%20WG%20Object%20Reference))
  ;[1 1 1] Initialize Map Event
  (bind _output_get (Variables|Default|SetMain%20Map%20WG WorldMap_WG))
  (bind _output_get_2 (Variables|Default|SetMap%20Reference (Variables|/Game/_ProjectContent/Widget/WorldMapSystem_MainWG.WorldMapSystem_MainWG_C|GetWorldMapSystem_WG _output_get)))
  (Default|Initialize _output_get_2 self)
  ;;[1 0.2812 0.2812] Wait for Character Module
  (Variables|Default|SetOriginalCharacterSize (Math|Vector2D|MakeVector2D 0.0 0.0))
  (bind _output_get_3 (Variables|Default|SetOriginalMapSize (Math|Vector2D|MakeVector2D (Math|Conversions|ToFloat(Integer) (Variables|/Game/_ProjectContent/Widget/WorldMapSystem_WG.WorldMapSystem_WG_C|GetMapSizeX (Variables|Default|GetMap%20Reference))) (Math|Conversions|ToFloat(Integer) (Variables|/Game/_ProjectContent/Widget/WorldMapSystem_WG.WorldMapSystem_WG_C|GetMapSizeY (Variables|Default|GetMap%20Reference))))))
  (Variables|/Game/_ProjectContent/Widget/WorldMapSystem_WG.WorldMapSystem_WG_C|SetOriginalMapSize (Variables|Default|GetMap%20Reference) _output_get_3))

(event Custom|OnInputModifySize
  (params (Increase? :type Boolean) (Percent :type Integer))
  (CallFunction|ModifyMapSize (+ 1.0 (* (/ (Math|Conversions|ToFloat(Integer) (Math|Integer|Clamp(Integer) Percent 0 100)) 1e+02) (Math|Conversions|ToFloat(Integer) (Math|Integer|SelectInt 1 -1 Increase?))))))

(event Custom|OnMapClick
  (params (Position :type Vector%202D%20Structure))
  (bind _location (CallFunction|MapPositiontoWorldLocation Position))
  (bind _out (CallFunction|TraceDownWorldLocation _location))
  (bind (_x _y _z) (Math|Vector|BreakVector _out))
  ;[1 1 1] On Map Click Event and Will Spawn Ship On Controller
  (Default|SpawnUnitonClient (Variables|Default|GetController) (Math|Vector|MakeVector _x _y (+ _z 3e+01))))

(event Custom|UpdateWGWorldLocation
  (bind _allmissileflag_arr (Variables|Default|GetAllMissileFlag_Arr))
  (bind _allflag_arr (Variables|Default|GetAllFlag_Arr))
  ;[1 1 1] Update Widget World Location
  (if (Utilities|Array|IsValidIndex _allflag_arr)
    (for _array_element _allflag_arr
      (Utilities|IsValid (Utilities|Struct|BreakShipFlag_Info _array_element)
        (:Is%20Valid
          (Utilities|Struct|SetmembersinShipFlag_Info _array_element (Variables|/Game/_ProjectContent/Widget/ShipFlag_WG.ShipFlag_WG_C|GetUnitWorldLocation (Utilities|Struct|BreakShipFlag_Info _array_element))))))
    (if (Utilities|Array|IsValidIndex _allmissileflag_arr)
      (for _array_element_2 _allmissileflag_arr
        (Utilities|IsValid (Utilities|Struct|BreakMissileFlag_Info _array_element_2)
          (:Is%20Valid
            (Utilities|Struct|SetmembersinMissileFlag_Info _array_element_2 (Variables|/Game/_ProjectContent/Widget/Missile_WG.Missile_WG_C|GetActorWorldLocation (Utilities|Struct|BreakMissileFlag_Info _array_element_2)))))))))

(event Custom|AddFlagOnBPC
  (params (Locaion :type Vector) (UnitRef :type Character%20Object%20Reference))
  ;[1 1 1] Add Flag On BpCWorld From Controller
  (CallFunction|AddFlag (Utilities|Struct|MakeShipFlag_Info Locaion 0 UnitRef)))

(event Custom|AddMissileFlagOnBPC
  (params (Location :type Vector) (ActorRef :type Actor%20Object%20Reference))
  ;[1 1 1] Add Missile Flag On BpCWorld From Controller
  (CallFunction|AddMissileFlag (Utilities|Struct|MakeMissileFlag_Info Location 0 ActorRef)))

(event Custom|AddCompoundFlagOnBPC
  (params (Location :type Vector) (ActorRef :type Actor%20Object%20Reference))
  ;[1 1 1] Add Compound Flag on BpCWorld From Controller
  (CallFunction|AddCompoundFlag (Utilities|Struct|MakeCompoundFlag_Info Location 0 ActorRef)))

(event Custom|UpdateUnitFlagVis
  (params (UnitInRangeArr :type Array%20of%20Actor%20Object%20References))
  ;[1 1 1] Update Unit Flag Visibility
  (bind _asrtscontroller (Utilities|Casting|CastToRTSController (Game|GetPlayerController 0)))
  (for _array_element (Variables|Default|GetAllFlag_Arr)
    (if (!= (Utilities|Array|FindItem UnitInRangeArr (.Unit_Ref (Utilities|Struct|BreakShipFlag_Info _array_element))) -1)
      (Widget|SetVisibility (.Widget (Utilities|Struct|BreakShipFlag_Info _array_element)) "Visible")
      (else
        (bind _shipside (CallFunction|GetUnitSide[Unit] (.Unit_Ref (Utilities|Struct|BreakShipFlag_Info _array_element))))
        (if (not (Utilities|Enum|Equal(Enum) _shipside (Variables|/Game/_ProjectContent/RTSController.RTSController_C|GetClient%20Side _asrtscontroller)))
          (Widget|SetVisibility (.Widget (Utilities|Struct|BreakShipFlag_Info _array_element)) "Hidden"))))))

(event EventTick
  (params (DeltaSeconds :type Float%20%28single-precision%29))
  ;[1 1 1] Event Tick
  (Utilities|FlowControl|Sequence
    (:then_0
      (CallFunction|UpdateFlagPositions)
      (CallFunction|UpdateFlagSize))
    (:then_1
      (Utilities|FlowControl|Delay 0.1)
      (CallFunction|UpdateWGWorldLocation))))

(fn GetMapHeight
  (return (Math|Float|Absolute(Float) (- (.x (Variables|Setting|GetLowerRightCorner)) (.x (Variables|Setting|GetUpperLeftCorner))))))

(fn GetMapWidth
  (return (Math|Float|Absolute(Float) (- (.y (Variables|Setting|GetLowerRightCorner)) (.y (Variables|Setting|GetUpperLeftCorner))))))

(fn ConvertLocationtoWorldLocation
  (params (Location :type Vector))
  (bind _upperleftcorner (Variables|Setting|GetUpperLeftCorner))
  (return (Math|Vector2D|MakeVector2D (Math|Float|Absolute(Float) (- (.y Location) (.y _upperleftcorner))) (Math|Float|Absolute(Float) (- (.x Location) (.x _upperleftcorner))))))

(fn LocationtoMapPosition
  (params (Location :type Vector) (WidgetSize :type Vector%202D%20Structure))
  (bind _out (CallFunction|ConvertLocationtoWorldLocation Location))
  (bind (_x _y) (Math|Vector2D|BreakVector2D WidgetSize))
  (bind _map_reference (Variables|Default|GetMap%20Reference))
  (return (Math|Vector2D|MakeVector2D (- (* (/ (.x _out) (CallFunction|GetMapWidth)) (Math|Conversions|ToFloat(Integer) (Variables|/Game/_ProjectContent/Widget/WorldMapSystem_WG.WorldMapSystem_WG_C|GetMapSizeX _map_reference))) (/ _x 2.0)) (- (* (/ (.y _out) (CallFunction|GetMapHeight)) (Math|Conversions|ToFloat(Integer) (Variables|/Game/_ProjectContent/Widget/WorldMapSystem_WG.WorldMapSystem_WG_C|GetMapSizeY _map_reference))) (/ _y 2.0)))))

(fn UpdateCharacterPostiononMap)

(fn ModifyMapSize
  (params (Multiply :type Float%20%28single-precision%29))
  (if (>= Multiply 0.0)
    (Variables|Default|SetCurrentSizeMultiplier (Math|Float|Clamp(Float) (* Multiply (Variables|Default|GetCurrentSizeMultiplier)) (Variables|Setting|GetMinZoom) (Variables|Setting|GetMaxZoom)))
    (Default|SetMapSize (Variables|Default|GetMap%20Reference) (Math|Float|Round (.x (* (Variables|Default|GetOriginalMapSize) (Variables|Default|GetCurrentSizeMultiplier)))) (Math|Float|Round (.y (* (Variables|Default|GetOriginalMapSize) (Variables|Default|GetCurrentSizeMultiplier)))))
    (CallFunction|UpdateFlagPositions)
    (return)
    (else
      (return))))

(fn MapOutOfBoundaries?
  (bind _returnvalue (Viewport|GetViewportSize))
  (bind _map_reference (Variables|Default|GetMap%20Reference))
  (bind _returnvalue_2 (Class|Widget|GetDesiredSize _map_reference))
  (return (or (> (.x _returnvalue_2) (.x _returnvalue)) (> (.y _returnvalue_2) (.y _returnvalue)))))

(fn AddFlag
  (params (Flag :type Ship%20Flag%20Info%20Structure))
  (bind (_worldlocation _unit_ref) (Utilities|Struct|BreakShipFlag_Info Flag))
  (bind _returnvalue (Utilities|Array|Add (Variables|Default|GetAllFlag_Arr) Flag))
  (LocalVariables|SetLocalIndex _returnvalue)
  (bind _ship_wgout (Default|AddUnittoMap (Variables|Default|GetMap%20Reference) self (CallFunction|LocationtoMapPosition _worldlocation (Variables|Default|GetFlagSize)) _unit_ref))
  (Utilities|Struct|SetmembersinShipFlag_Info (Utilities|Array|Get(acopy) (Variables|Default|GetAllFlag_Arr) (LocalVariables|GetLocalIndex)) _ship_wgout)
  (CallFunction|SetFlagRefonUnit[OutCast] _unit_ref _ship_wgout))

(fn MapPositiontoWorldLocation
  (params (Position :type Vector%202D%20Structure))
  (bind _map_reference (Variables|Default|GetMap%20Reference))
  (bind _upperleftcorner (Variables|Setting|GetUpperLeftCorner))
  (LocalVariables|SetLocalPercentage%20in%20X (/ (.x Position) (Math|Conversions|ToFloat(Integer) (Variables|/Game/_ProjectContent/Widget/WorldMapSystem_WG.WorldMapSystem_WG_C|GetMapSizeX _map_reference))))
  (LocalVariables|SetLocalPercentage%20in%20Y (/ (.y Position) (Math|Conversions|ToFloat(Integer) (Variables|/Game/_ProjectContent/Widget/WorldMapSystem_WG.WorldMapSystem_WG_C|GetMapSizeY _map_reference))))
  (return (Math|Vector|MakeVector (- (.x _upperleftcorner) (* (CallFunction|GetMapHeight) (LocalVariables|GetLocalPercentage%20in%20Y))) (+ (.y _upperleftcorner) (* (CallFunction|GetMapWidth) (LocalVariables|GetLocalPercentage%20in%20X))) -5e+02)))

(fn TraceDownWorldLocation
  (params (In :type Vector))
  (LocalVariables|SetLocal_In In)
  (bind (_outhit _returnvalue) (Collision|LineTraceByChannel (Math|Vector|MakeVector (.x (LocalVariables|GetLocal_In)) (.y (LocalVariables|GetLocal_In)) (Variables|Default|GetTraceDownHeight)) (LocalVariables|GetLocal_In) "TraceTypeQuery4" false 0 "None"))
  (if _returnvalue
    (return (.Location (Collision|BreakHitResult _outhit)))
    (else
      (return (LocalVariables|GetLocal_In)))))

(fn UpdateFlagPositions
  (for _array_element (Variables|Default|GetAllFlag_Arr)
    (Utilities|IsValid (Utilities|Struct|BreakShipFlag_Info _array_element)
      (:Is%20Valid
        (Class|Widget|SetRenderTranslation (Utilities|Struct|BreakShipFlag_Info _array_element) (CallFunction|LocationtoMapPosition (Variables|/Game/_ProjectContent/Widget/ShipFlag_WG.ShipFlag_WG_C|GetUnitWorldLocation (Utilities|Struct|BreakShipFlag_Info _array_element)) (Variables|Default|GetFlagSize))))))
  (for _array_element_2 (Variables|Default|GetAllMissileFlag_Arr)
    (Utilities|IsValid (Utilities|Struct|BreakMissileFlag_Info _array_element_2)
      (:Is%20Valid
        (Class|Widget|SetRenderTranslation (Utilities|Struct|BreakMissileFlag_Info _array_element_2) (CallFunction|LocationtoMapPosition (Variables|/Game/_ProjectContent/Widget/Missile_WG.Missile_WG_C|GetActorWorldLocation (Utilities|Struct|BreakMissileFlag_Info _array_element_2)) "(X=35.000000,Y=35.000000)")))))
  (for _array_element_3 (Variables|Default|GetAllCompoundFlag_Arr)
    (Utilities|IsValid (.Widget (Utilities|Struct|BreakCompoundFlag_Info _array_element_3))
      (:Is%20Valid
        (Class|Widget|SetRenderTranslation (.Widget (Utilities|Struct|BreakCompoundFlag_Info _array_element_3)) (CallFunction|LocationtoMapPosition (.WorldLocation (Utilities|Struct|BreakCompoundFlag_Info _array_element_3)) (Class|Widget|GetDesiredSize (.Widget (Utilities|Struct|BreakCompoundFlag_Info _array_element_3))))))))
  (return))

(fn SetFlagRefonUnit[OutCast]
  (params (Unit%20Ref :type Character%20Object%20Reference) (UnitFlagRef :type Ship%20Flag%20WG%20Object%20Reference))
  (bind _ass_fs_442_bp (Utilities|Casting|CastToS_FS-442_BP Unit%20Ref))
  (Variables|/Game/_ProjectContent/_Blueprints/Character/Ship/S_FS-442_BP.S_FS-442_BP_C|SetShip%20Flag%20WG _ass_fs_442_bp UnitFlagRef))

(fn UpdateFlagSize
  (Utilities|FlowControl|Sequence
    (:then_0
      (for _array_element (Variables|Default|GetAllFlag_Arr)
        (Utilities|IsValid (Utilities|Struct|BreakShipFlag_Info _array_element)
          (:Is%20Valid
            (Default|UpdateSize (Utilities|Struct|BreakShipFlag_Info _array_element) (Variables|/Game/_ProjectContent/Widget/WorldMapSystem_WG.WorldMapSystem_WG_C|GetCurrentSizeMultiplier (Variables|Default|GetMap%20Reference)))))))))

(fn SetFlagRefonMissile[OutCast]
  (params (ActorRef :type Actor%20Object%20Reference) (ActorFlagRef :type Missile%20WG%20Object%20Reference))
  (bind _asharpoon_missile_bp (Utilities|Casting|CastToHarpoon_Missile_BP ActorRef))
  (Variables|/Game/_ProjectContent/_Blueprints/Character/Weapon/Harpoon_Missile_BP.Harpoon_Missile_BP_C|SetFlagWG _asharpoon_missile_bp ActorFlagRef))

(fn AddMissileFlag
  (params (MissileFlag :type Missile%20Flag%20Info%20Structure))
  (bind (_worldlocation _actor_ref) (Utilities|Struct|BreakMissileFlag_Info MissileFlag))
  (bind _returnvalue (Utilities|Array|Add (Variables|Default|GetAllMissileFlag_Arr) MissileFlag))
  (LocalVariables|SetLocalIndex _returnvalue)
  (bind _missilewgout (Default|AddMissiletoMap (Variables|Default|GetMap%20Reference) self (CallFunction|LocationtoMapPosition _worldlocation (Variables|Default|GetFlagSize)) _actor_ref))
  (Utilities|Struct|SetmembersinMissileFlag_Info (Utilities|Array|Get(acopy) (Variables|Default|GetAllMissileFlag_Arr) (LocalVariables|GetLocalIndex)) _missilewgout)
  (CallFunction|SetFlagRefonMissile[OutCast] _actor_ref _missilewgout))

(fn DetonateMissileWG
  (params (MissileWG_Ref :type Missile%20WG%20Object%20Reference))
  (bind _allmissileflag_arr (Variables|Default|GetAllMissileFlag_Arr))
  (for (_array_element _array_index) _allmissileflag_arr
    (if (== (Utilities|Struct|BreakMissileFlag_Info _array_element) MissileWG_Ref)
      (Widget|RemovefromParent (Utilities|Struct|BreakMissileFlag_Info _array_element))
      (Utilities|Array|RemoveIndex _allmissileflag_arr _array_index)
      (return))))

(fn UpdateFlagVisibility)

(fn AddCompoundFlag
  (params (CompoundFlag :type Compound%20Flag%20Info%20Structure))
  (bind (_worldlocation _actorref) (Utilities|Struct|BreakCompoundFlag_Info CompoundFlag))
  (bind _returnvalue (Utilities|Array|Add (Variables|Default|GetAllCompoundFlag_Arr) CompoundFlag))
  (LocalVariables|SetLocalIndex _returnvalue)
  (bind _compoundwgout (Default|AddCompoundtoMap (Variables|Default|GetMap%20Reference) self (CallFunction|LocationtoMapPosition _worldlocation (Variables|Default|GetFlagSize)) _actorref))
  (Utilities|Struct|SetmembersinCompoundFlag_Info (Utilities|Array|Get(acopy) (Variables|Default|GetAllCompoundFlag_Arr) (LocalVariables|GetLocalIndex)) _compoundwgout)
  (bind _ascompound_tag_bp (Utilities|Casting|CastToCompound_Tag_BP _actorref))
  (Variables|/Game/_ProjectContent/_Blueprints/Compound_Tag_BP.Compound_Tag_BP_C|SetCompoundWG _ascompound_tag_bp _compoundwgout))