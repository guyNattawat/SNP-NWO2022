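; Spline patrol path actor that provides a moving target point, apparently for EnemyAIBoat_BP enemy boats.
; A timeline starts on BeginPlay, sweeps a Cube along the spline's length, stores its world position in Location, and replays after a short delay.
; Pause and Continue events stop and resume the motion.
; Sphere overlaps with enemy boats set and clear an OverlappingAI flag.
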(event OnComponentBeginOverlap(Sphere)
  (params (OverlappedComponent :type Primitive%20Component%20Object%20Reference) (OtherActor :type Actor%20Object%20Reference) (OtherComp :type Primitive%20Component%20Object%20Reference) (OtherBodyIndex :type Integer) (bFromSweep :type Boolean) (SweepResult :type Hit%20Result%20Structure%20%28by%20ref%29))
  (Utilities|Casting|CastToEnemyAIBoat_BP OtherActor)
  (Variables|Default|SetOverlappingAI? true))

(event OnComponentEndOverlap(Sphere)
  (params (OverlappedComponent :type Primitive%20Component%20Object%20Reference) (OtherActor :type Actor%20Object%20Reference) (OtherComp :type Primitive%20Component%20Object%20Reference) (OtherBodyIndex :type Integer))
  (Utilities|Casting|CastToEnemyAIBoat_BP OtherActor)
  (Variables|Default|SetOverlappingAI? false))

(event Custom|Continue
  (bind _newtrack_0 (Timeline|Timeline_0 Play)
    (:Update
      (Variables|Default|SetLocation (Spline|GetLocationatDistanceAlongSpline (Variables|Default|GetSpline) (Math|Float|Lerp 0.0 (Spline|GetSplineLength (Variables|Default|GetSpline)) _newtrack_0) "World"))
      (Transformation|SetWorldLocation (Variables|Default|GetCube) (Spline|GetLocationatDistanceAlongSpline (Variables|Default|GetSpline) (Math|Float|Lerp 0.0 (Spline|GetSplineLength (Variables|Default|GetSpline)) _newtrack_0) "World") false false))
    (:Finished
      (Utilities|FlowControl|Delay 0.2)
      (Timeline|Timeline_0 PlayFromStart))))

(event Custom|Pause
  (bind _newtrack_0 (Timeline|Timeline_0 Stop)
    (:Update
      (Variables|Default|SetLocation (Spline|GetLocationatDistanceAlongSpline (Variables|Default|GetSpline) (Math|Float|Lerp 0.0 (Spline|GetSplineLength (Variables|Default|GetSpline)) _newtrack_0) "World"))
      (Transformation|SetWorldLocation (Variables|Default|GetCube) (Spline|GetLocationatDistanceAlongSpline (Variables|Default|GetSpline) (Math|Float|Lerp 0.0 (Spline|GetSplineLength (Variables|Default|GetSpline)) _newtrack_0) "World") false false))
    (:Finished
      (Utilities|FlowControl|Delay 0.2)
      (Timeline|Timeline_0 PlayFromStart))))

(event EventBeginPlay
  (bind _newtrack_0 (Timeline|Timeline_0 Play)
    (:Update
      (Variables|Default|SetLocation (Spline|GetLocationatDistanceAlongSpline (Variables|Default|GetSpline) (Math|Float|Lerp 0.0 (Spline|GetSplineLength (Variables|Default|GetSpline)) _newtrack_0) "World"))
      (Transformation|SetWorldLocation (Variables|Default|GetCube) (Spline|GetLocationatDistanceAlongSpline (Variables|Default|GetSpline) (Math|Float|Lerp 0.0 (Spline|GetSplineLength (Variables|Default|GetSpline)) _newtrack_0) "World") false false))
    (:Finished
      (Utilities|FlowControl|Delay 0.2)
      (Timeline|Timeline_0 PlayFromStart))))

(fn ConstructionScript)