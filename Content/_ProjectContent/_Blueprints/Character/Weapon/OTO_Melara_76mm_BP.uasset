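; Automated OTO Melara 76mm naval gun turret that engages other-side pawns while its ship's weapon system state is on.
; Each tick it picks the nearest target in line of sight, slews the yaw-clamped turret and sets barrel pitch from a low-arc ballistic solution.
; Once aligned and cooled down, it spawns server-side projectiles with cone spread based on ship velocity, using limited ammo and a timed reload.
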(event Custom|EventUpdateOnServer
  (params (DeltaSec :type Float%20%28single-precision%29))
  (Private|FindBestTarget)
  (Variables|Private|GetTarget
    (:then
      (Private|UpdateTurretRotation DeltaSec)
      (Private|UpdateFire))
    (:else)))

(event Custom|Reload
  (Variables|Default|SetReload? true)
  (Utilities|FlowControl|Delay (Variables|Ability|GetReloadSpeed))
  (Variables|Ability|SetCurrentAmmo (Variables|Ability|GetMaxAmmo))
  (Variables|Default|SetReload? false))

(event Custom|UpdateWeaponDetails)

(event Custom|FireOnServer
  (bind _firepos (Variables|Default|GetFirePos))
  (if (> (Variables|Ability|GetCurrentAmmo) 0)
    (Variables|Ability|SetCurrentAmmo (- (Variables|Ability|GetCurrentAmmo) 1))
    (if (Networking|IsServer)
      (Variables|Private|SetTimeOfLastFire (GameState|GetServerWorldTimeSeconds (Game|GetGameState)))
      (Utilities|FlowControl|Sequence
        (:then_0
          (if (> (.x (Transformation|GetVelocity (Variables|Default|GetShip_Owner))) 0.0)
            (Variables|Ability|SetAccuracy 0.2)
            (else
              (Variables|Ability|SetAccuracy 0.5)))
          (Game|SpawnActorfromClass "/Game/_ProjectContent/_Blueprints/BulletProjectile.BulletProjectile_C" (Math|Transform|MakeTransform (.location (Transformation|GetWorldTransform _firepos)) (Math|Conversions|RotationFromXVector (Math|Random|RandomUnitVectorinConeinDegrees (Math|Vector|GetForwardVector _firepos) (Variables|Ability|GetAccuracy))) "0.050000,0.050000,0.050000") "Undefined" 0 0))))
    (elif (not (Variables|Default|GetReload?))
      (CallFunction|Reload))))

(event EventBeginPlay
  (Variables|Ability|SetCurrentAmmo (Variables|Ability|GetMaxAmmo))
  (Utilities|FlowControl|Delay 0.2)
  (CallFunction|UpdateWeaponDetails))

(event EventTick
  (params (DeltaSeconds :type Float%20%28single-precision%29))
  (Utilities|FlowControl|Sequence
    (:then_0
      (bind _weaponsystemstate (CallFunction|GetShipCommand (Variables|Default|GetShip_Owner)))
      (if _weaponsystemstate
        (CallFunction|EventUpdateonServer DeltaSeconds)))))

(fn ConstructionScript)

(fn FindBestTarget
  (bind _turret_top (Variables|Default|Getturret_Top))
  (bind _returnvalue (Transformation|GetWorldLocation _turret_top))
  (Utilities|FlowControl|Sequence
    (:then_0
      (LocalVariables|SetBestDistance%20%28Local%29 (+ (Variables|Contants|GetSensingRange) 1.0))
      (bind _outactors (Collision|SphereOverlapActors (Transformation|GetActorLocation) (Variables|Contants|GetSensingRange) (Utilities|Array|MakeArray "ObjectTypeQuery3") "/Script/Engine.Actor" (Variables|Default|GetActors%20to%20Ignore%20Arr)))
      ;[1 1 1] Compare Client Side
      (for _array_element _outactors
        (bind _shipside (CallFunction|GetShipSide _array_element))
        (if (Utilities|Enum|NotEqual(Enum) _shipside (Variables|Default|GetOwnerSide))
          (bind _output_get (LocalVariables|SetCurrentTarget%20%28Local%29 _array_element))
          (bind _output_get_2 (LocalVariables|SetCurrentDistance%20%28Local%29 (Transformation|GetDistanceTo _output_get self)))
          (if (or (< _output_get_2 (LocalVariables|GetBestDistance%20%28Local%29)) (not (Utilities|IsValid (LocalVariables|GetBestTarget%20%28Local%29)))) ; Is This closest target so far?
            (bind _result (CallFunction|HasLineOfSight (Math|Vector|MakeVector (.x _returnvalue) (.y _returnvalue) 3e+01) (Math|Vector|MakeVector (.x (Transformation|GetActorLocation (LocalVariables|GetCurrentTarget%20%28Local%29))) (.y (Transformation|GetActorLocation (LocalVariables|GetCurrentTarget%20%28Local%29))) 7e+01) (Variables|Default|GetActors%20to%20Ignore%20Arr)))
            (if _result
              (LocalVariables|SetBestTarget%20%28Local%29 (LocalVariables|GetCurrentTarget%20%28Local%29))
              (LocalVariables|SetBestDistance%20%28Local%29 (LocalVariables|GetCurrentDistance%20%28Local%29))))))
      (Variables|Private|SetTarget (LocalVariables|GetBestTarget%20%28Local%29)))))

(fn UpdateTurretRotation
  (params (DeltaSeconds :type Float%20%28single-precision%29))
  (bind _turret_base (Variables|Default|Getturret_Base))
  (bind _turret_top (Variables|Default|Getturret_Top))
  (bind _rotation_speed (Variables|Ability|GetRotation%20Speed))
  (bind _turret_top_2 (Variables|Default|Getturret_Top))
  (bind _turret_barrel (Variables|Default|Getturret_Barrel))
  (bind _target (Variables|Private|GetTarget))
  (bind _deltaseconds (LocalVariables|GetDeltaseconds))
  (bind _returnvalue (Transformation|GetWorldTransform _turret_base))
  (bind _returnvalue_2 (Transformation|GetWorldRotation _turret_barrel))
  (bind _returnvalue_3 (Transformation|GetWorldLocation _turret_top_2))
  (bind _returnvalue_4 (Transformation|GetActorLocation _target))
  (bind _returnvalue_5 (Transformation|GetWorldRotation _turret_top))
  (bind _returnvalue_6 (Math|Rotator|FindLookatRotation _returnvalue_3 _returnvalue_4))
  (bind _returnvalue_7 (Class|KismetMathLibrary|RInterptoConstant _returnvalue_5 _returnvalue_6 _deltaseconds _rotation_speed))
  (bind _returnvalue_8 (Math|Transform|InverseTransformRotation _returnvalue _returnvalue_7))
  (Transformation|SetRelativeRotation (Variables|Default|Getturret_Top) (Math|Rotator|MakeRotator (.roll _returnvalue_8) 0.0 (Math|Float|ClampAngle (.yaw _returnvalue_8) -9e+01 9e+01)) false false)
  (bind _angleresult (CallFunction|FindAngle))
  (Transformation|SetWorldRotation _turret_barrel (Math|Rotator|MakeRotator (.roll _returnvalue_2) _angleresult (.yaw _returnvalue_2)) false false))

(fn OnRepOwnerSide)

(fn TurretColorSet)

(fn UpdateFire
  (if (> (- (Utilities|Time|GetGameTimeinSeconds) (Variables|Private|GetTimeOfLastFire)) (Variables|Private|GetRateOfFire)) ; Have Rate of Fire Cooled Down?
    (if (> (Math|Vector|DotProduct (Math|Vector|GetUnitDirection(Vector) (Transformation|GetWorldLocation (Variables|Default|Getturret_Top)) (Transformation|GetActorLocation (Variables|Private|GetTarget))) (Math|Vector|GetForwardVector (Variables|Default|Getturret_Top))) 0.99) ; Is the turret facing to target?
      (CallFunction|FireonServer))))

(fn FindAngle
  (bind _target (Variables|Private|GetTarget))
  (bind _velocity (Variables|Ability|GetVelocity))
  (bind _gravity (Variables|Ability|GetGravity))
  (bind _turret_barrel (Variables|Default|Getturret_Barrel))
  (bind _returnvalue (Transformation|GetSocketLocation _turret_barrel "FireSocket"))
  (bind _returnvalue_2 (Transformation|GetActorLocation _target))
  (bind _returnvalue_3 (Math|Float|Square _velocity))
  (bind _returnvalue_4 (Math|Float|Square _returnvalue_3))
  (bind _returnvalue_5 (- (.z _returnvalue_2) (.z _returnvalue)))
  (bind _returnvalue_6 (- (.x _returnvalue_2) (.x _returnvalue)))
  (bind _returnvalue_7 (- (.y _returnvalue_2) (.y _returnvalue)))
  (bind _returnvalue_8 (Math|Vector2D|Vector2DLength (Math|Vector2D|MakeVector2D _returnvalue_6 _returnvalue_7)))
  (bind _returnvalue_9 (* _returnvalue_5 _returnvalue_3))
  (bind _returnvalue_10 (Math|Float|Square _returnvalue_8))
  (bind _returnvalue_11 (* _returnvalue_9 2.0))
  (bind _returnvalue_12 (* _returnvalue_8 _gravity))
  (bind _returnvalue_13 (* _returnvalue_10 _gravity))
  (bind _returnvalue_14 (+ _returnvalue_13 _returnvalue_11))
  (bind _returnvalue_15 (* _returnvalue_14 _gravity))
  (bind _returnvalue_16 (- _returnvalue_4 _returnvalue_15))
  (bind _returnvalue_17 (Math|Float|Sqrt _returnvalue_16))
  (return (Math|Float|Min(Float) (Class|KismetMathLibrary|DegAtan (/ (+ _returnvalue_17 _returnvalue_3) _returnvalue_12)) (Class|KismetMathLibrary|DegAtan (/ (- _returnvalue_3 _returnvalue_17) _returnvalue_12)))))

(fn OnRepTimeOfLastFire)

(fn GetShipCommand
  (params (Ship%20Ref :type Character%20Object%20Reference)))