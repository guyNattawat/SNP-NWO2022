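; Test bullet actor that flies along its forward direction and destroys itself after about 20 seconds.
; Each Tick moves the root by the forward vector with Z zeroed, scaled by a fixed speed and delta time, without sweep.
; The lifetime comes from a Delay in the Tick chain that leads to DestroyActor.
; The graph contains no hit or damage logic.
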(event EventTick
  (params (DeltaSeconds :type Float%20%28single-precision%29))
  (Transformation|SetWorldLocation (Variables|Default|GetDefaultSceneRoot) (+ (Transformation|GetWorldLocation (Variables|Default|GetDefaultSceneRoot)) (* (* (* (Math|Vector|GetForwardVector (Variables|Default|GetDefaultSceneRoot)) "1.000000,1.000000, 0") 2.5e+03) (Utilities|Time|GetWorldDeltaSeconds))) false false)
  (Utilities|FlowControl|Delay 2e+01)
  (Actor|DestroyActor))

(fn ConstructionScript)